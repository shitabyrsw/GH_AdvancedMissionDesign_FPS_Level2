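; BP_Target is a damageable target that shows the damage it takes as floating text and triggers the player's HUD hit marker.
; AnyDamage adds damage to a running score, shows it on a TextRender component and calls the hit marker message on the first player's HUD.
; It also sets a one-second timer event that hides the text and clears the score.
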(event Custom|Countdown
  ;[1 1 1] Hide Text
  (Development|SetHiddeninGame (Variables|Default|GetTextRender) true false)
  (Variables|Default|SetDmgScore 0.0))

(event Game|Damage|EventAnyDamage
  (params (Damage :type Float%20%28single-precision%29) (DamageType :type Damage%20Type%20Object%20Reference) (InstigatedBy :type Controller%20Object%20Reference) (DamageCauser :type Actor%20Object%20Reference))
  (Utilities|FlowControl|Sequence
    (:then_0
      ;[1 1 1] Update Text
      (bind _output_get (Variables|Default|SetDmgScore (+ (Variables|Default|GetDmgScore) Damage)))
      (Rendering|Components|TextRender|SetText (Variables|Default|GetTextRender) (Utilities|Text|FormatText "{Damage} dmg" _output_get)))
    (:then_1
      ;[1 1 1] Show Text
      (Development|SetHiddeninGame (Variables|Default|GetTextRender) false false))
    (:then_2
      ;[1 1 1] Hide Text
      (bind _returnvalue (Utilities|Time|SetTimerbyEvent (delegate Custom|Countdown) 1.0))
      (Variables|Default|SetDmgTimer _returnvalue))
    (:then_3
      ;[1 1 1] Show Hit Marker
      (Class|BPIHUD|ShowHitMarker(Message) (HUD|GetHUD (Game|GetPlayerController 0))))))

(fn ConstructionScript)