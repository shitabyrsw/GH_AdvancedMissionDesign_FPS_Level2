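; Physics-driven hovering movement component for BP_Master_Enemy owners, which simulates the capsule without gravity and pushes it toward destinations.
; SetDestination line-traces to choose direct flight or a navmesh path, lifts points to hover height above traced surfaces and starts a five-second timeout.
; Tick applies distance-scaled thrust, adds torque to face velocity and stay upright unless stalled, and advances path points.
; Arrival and timeout fire dispatchers.
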(event Custom|Pathfinding%20Failed
  ;[1 1 1] Pathfinding Failed
  (CallFunction|MoveDirectlytoDestination))

(event Custom|MoveDirectlyToDestination
  ;[1 1 1] Move Directly to Destination
  (Variables|Movement|SetCurrentDestination (Variables|Movement|GetAdjustedFinalDestination)))

(event Custom|MoveAlongPath
  (params (Path :type Array%20of%20Vectors))
  ;[1 1 1] Move Along path
  (Variables|Movement|Pathfinding|SetCurrentPath Path)
  (bind _adjustedlocation (Utilities|AccountforHoverHeight (Utilities|Array|Get(acopy) (Variables|Movement|Pathfinding|GetCurrentPath))))
  (Variables|Movement|SetCurrentDestination _adjustedlocation))

(event Custom|SetDestination
  (params (Destination :type Vector))
  ;[1 1 1] New Destination
  (bind _returnvalue (Utilities|Time|SetTimerbyEvent (delegate Custom|TimeoutMovement) 5.0))
  (Variables|Default|SetMovementTimeout _returnvalue)
  (Variables|Movement|SetFinalDestination Destination)
  ;[1 1 1] Adjust Destination Height
  (bind _adjustedlocation (Utilities|AccountforHoverHeight (Variables|Movement|GetFinalDestination)))
  (Variables|Movement|SetAdjustedFinalDestination _adjustedlocation)
  (Variables|Movement|SetStartingPosition (Transformation|GetActorLocation (Variables|Default|GetOwningEnemy)))
  ;[1 1 1] Check should use path
  (bind _returnvalue_2 (Collision|LineTraceForObjects (Variables|Movement|GetStartingPosition) (Variables|Movement|GetFinalDestination) (Utilities|GetTraceObjectTypes) false 0 (.TraceType (Utilities|GetDebug))))
  (if _returnvalue_2
    (Variables|Movement|Pathfinding|SetbUsingPath true)
    (bind _floor (Utilities|FindFloor))
    ;[1 1 1] Find path
    (bind _returnvalue_3 (Class|NavigationSystemV1|FindPathtoLocationSynchronously _floor (Variables|Movement|GetFinalDestination) (Variables|Default|GetOwningEnemy) 0))
    (if (Utilities|IsValid _returnvalue_3)
      (CallFunction|MoveAlongPath (Variables|/Script/NavigationSystem.NavigationPath|GetPathPoints _returnvalue_3))
      (else
        (CallFunction|DebugLog "Invalid Path" "NewEnumerator1" "None" false)
        (CallFunction|PathfindingFailed)))
    (else
      (CallFunction|MoveDirectlytoDestination))))

(event Custom|GetNextPathPoint
  ;[1 1 1] Get Next point on path
  (bind _result (Math|Integer|IncrementInt (Variables|Movement|Pathfinding|GetCurrentPathIndex))
    (:%20%20
      (if (Utilities|Array|IsValidIndex (Variables|Movement|Pathfinding|GetCurrentPath) _result)
        (bind _adjustedlocation (Utilities|AccountforHoverHeight (Utilities|Array|Get(acopy) (Variables|Movement|Pathfinding|GetCurrentPath) (Variables|Movement|Pathfinding|GetCurrentPathIndex))))
        (Variables|Movement|SetCurrentDestination _adjustedlocation)
        (else
          (Variables|Movement|Pathfinding|SetCurrentPathIndex 0)
          (Variables|Movement|Pathfinding|SetbUsingPath false)
          (Utilities|Array|Clear (Variables|Movement|Pathfinding|GetCurrentPath))
          (CallFunction|ReachedDestination))))))

(event Custom|ReachedDestination
  ;[1 1 1] Destination Reached
  (Variables|Movement|SetCurrentDestination "0, 0, 0")
  (Utilities|Time|ClearandInvalidateTimerbyHandle (Variables|Default|GetMovementTimeout))
  (Default|CallDestinationReached))

(event Custom|StallRotation
  (params (Duration :type Float%20%28single-precision%29))
  ;[1 1 1] Tick
  ;;[1 1 1] Add Tourqe to face velocity & stay upright
  ;;;[1 1 1] Stall Rotation tourqe
  (Variables|Physics|SetRotaionStall true)
  (Utilities|FlowControl|Delay Duration)
  (Variables|Physics|SetRotaionStall false))

(event Custom|HeightTrace
  ;[1 1 0] Height Trace
)

(event Custom|TimeoutMovement
  ;[1 1 1] New Destination
  (Utilities|Time|ClearandInvalidateTimerbyHandle (Variables|Default|GetMovementTimeout))
  (Default|CallPathfindingFailed))

(event EventBeginPlay
  ;[1 1 1] Begin Play
  (bind _asbp_master_enemy (Utilities|Casting|CastToBP_Master_Enemy (Components|GetOwner))
    (:then
      (Variables|Default|SetOwningEnemy _asbp_master_enemy)
      (Utilities|FlowControl|Sequence
        (:then_0
          ;[1 1 1] Setup Comp
          (Variables|Movement|SetCurrentDestination (Transformation|GetActorLocation (Variables|Default|GetOwningEnemy))) ; Inital Position
        )
        (:then_1
          ;[1 1 1] Setup Charachter
          (Physics|SetSimulatePhysics (Utilities|GetCapsuleComponent) true)
          (Physics|SetEnableGravity (Utilities|GetCapsuleComponent) false)
          (Variables|/Script/Engine.CharacterMovementComponent|SetGravityScale (Variables|/Script/Engine.Character|GetCharacterMovement (Variables|Default|GetOwningEnemy)) 0.0)
          (Class|PrimitiveComponent|SetLinearDamping (Utilities|GetCapsuleComponent) (Variables|Physics|GetLinearDamping))
          (Class|PrimitiveComponent|SetAngularDamping (Utilities|GetCapsuleComponent) (Variables|Physics|GetAngularDamping)))))
    (:CastFailed
      (CallFunction|DebugLog "Physics Movement Comp only supported on master enemy class" "NewEnumerator0" "None" false))))

(event EventTick
  (params (DeltaSeconds :type Float%20%28single-precision%29))
  (bind _returnvalue (CallFunction|CalculateThrust))
  (bind (_currentdestination _finallocaiton) (Utilities|HasReachedDestination))
  (bind _capsule_component (Utilities|GetCapsuleComponent))
  ;[1 1 1] Tick
  (Utilities|FlowControl|Sequence
    (:then_0
      ;;[1 1 1] Add Movement thrust
      (if (not (.FinalLocaiton (Utilities|HasReachedDestination)))
        (Physics|AddForce (Utilities|GetCapsuleComponent) (Math|Vector|MakeVector (.x _returnvalue) (.y _returnvalue) (.z _returnvalue)) "None" true)))
    (:then_1
      ;;[1 1 1] Add Tourqe to face velocity & stay upright
      (if (Variables|Physics|GetbOrientToVelocity)
        (if (not (Variables|Physics|GetRotaionStall))
          ;;;[1 1 1] Yaw
          (Class|PrimitiveComponent|AddTorqueinDegrees (Utilities|GetCapsuleComponent) (Math|Vector|MakeVector 0.0 0.0 (+ (* (Math|Vector|DotProduct (Math|Vector|GetRightVector (Transformation|GetWorldRotation _capsule_component)) (Math|Vector|Normalize (Transformation|GetComponentVelocity _capsule_component))) 5e+04) (Math|Random|RandomFloatinRange 0.0 1e+03))) "None" true)
          ;;;[1 1 1] Pitch
          (Class|PrimitiveComponent|AddTorqueinDegrees (Utilities|GetCapsuleComponent) (Math|Vector|MakeVector (* (Math|Vector|DotProduct "0.000000,1.000000,0.000000" (Math|Vector|GetUpVector (Utilities|GetCapsuleComponent))) 5e+03) 0.0 0.0) "None" true)
          ;;;[1 1 1] Roll
          (Class|PrimitiveComponent|AddTorqueinDegrees (Utilities|GetCapsuleComponent) (Math|Vector|MakeVector 0.0 (* (Math|Vector|DotProduct "-1.000000, 0,0.000000" (Math|Vector|GetUpVector (Utilities|GetCapsuleComponent))) 5e+03) 0.0) "None" true))))
    (:then_2
      ;;[1 1 1] Check if reached Destination
      (if _finallocaiton
        (CallFunction|ReachedDestination)
        (elif _currentdestination
          (if (Variables|Movement|Pathfinding|GetbUsingPath)
            (CallFunction|GetNextPathPoint)
            (else
              (CallFunction|ReachedDestination))))))
    (:then_3
      (CallFunction|HeightTrace))))

(fn CalculateThrust
  (bind _currentdestination (Variables|Movement|GetCurrentDestination))
  (bind _startingposition (Variables|Movement|GetStartingPosition))
  (bind _returnvalue (Math|Vector|Distance(Vector) _startingposition _currentdestination))
  (return (* (Math|Vector|GetUnitDirection(Vector) (Transformation|GetActorLocation (Variables|Default|GetOwningEnemy)) (Variables|Movement|GetCurrentDestination)) (* (Variables|Physics|GetThrustForce) (Math|Float|Clamp(Float) (/ (- _returnvalue (- _returnvalue (Math|Vector|Distance(Vector) (Transformation|GetActorLocation (Variables|Default|GetOwningEnemy)) (Variables|Movement|GetCurrentDestination)))) _returnvalue) 0.5)))))