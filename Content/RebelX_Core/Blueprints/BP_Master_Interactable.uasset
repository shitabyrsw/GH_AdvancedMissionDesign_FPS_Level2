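; BP_Master_Interactable is the base actor for interactable objects, exposing queries for ammo, health, scene info, interaction type, consumability and crosshair prompt text.
; Every query returns a false, empty or default value, leaving real data to be supplied by overrides.
; AttemptConsumeInteractable destroys the actor without checking consumability, while ActivateSceneObject and the construction script are empty.
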(event EventActivateSceneObject)

(event EventAttemptConsumeInteractable
  (Actor|DestroyActor))

(fn ConstructionScript)

(fn GetAmmoInfo
  (return false "NewEnumerator0"))

(fn GetCrosshairPrompt
  (return "" ""))

(fn GetHealthInfo
  (return false 0.0))

(fn GetInteractionType
  (return false "NewEnumerator0"))

(fn GetIsConsumeable
  (return false))

(fn GetSceneInfo
  (return false))