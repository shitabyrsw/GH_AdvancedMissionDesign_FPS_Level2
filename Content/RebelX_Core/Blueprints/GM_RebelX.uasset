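; RebelX game mode that opens a level kill-enemies door based on counts of living enemies.
; Every Tick it checks whether AmountAlive2 equals one, then, through a DoOnce, calls OpenDoor on the first L2_BP_Door_KillEnemies actor found.
; A similar AmountAlive1 check for the same door class is disconnected and never runs.
; Neither counter is updated in this graph.
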(event EventTick
  (params (DeltaSeconds :type Float%20%28single-precision%29))
  (if (== (Variables|Default|GetAmountAlive_2) 1)
    (Utilities|FlowControl|DoOnce false
      (:Completed
        (bind _outactors (Actor|GetAllActorsOfClass "/Game/L2_BluePrint/L2_BP_Door_KillEnemies.L2_BP_Door_KillEnemies_C"))
        (Default|OpenDoor (Utilities|Array|Get(acopy) _outactors))))))

(fn ConstructionScript)