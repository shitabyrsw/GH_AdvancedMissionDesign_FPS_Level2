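; Anim notify that deals knife melee damage at the moment it fires in the attack animation.
; It sphere-traces through the mesh's knife socket along the owner's camera forward vector, fetched through an interface message, ignoring the owner.
; A hit applies flat damage to the hit actor with the owner as causer and returns true; a miss returns false.
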(fn ReceivedNotify
  (params (MeshComp :type Skeletal%20Mesh%20Component%20Object%20Reference) (Animation :type Anim%20Sequence%20Base%20Object%20Reference) (EventReference :type Anim%20Notify%20Event%20Reference%20Structure%20%28by%20ref%29))
  (bind _returnvalue (Transformation|GetSocketLocation MeshComp "Socket_Knife"))
  (bind _returnvalue_2 (Components|GetOwner MeshComp))
  (bind _returnvalue_3 (Class|BPILPAMGPCH|LPAMG-GetCameraComponent(Message) (Components|GetOwner MeshComp)))
  (bind (_outhit _returnvalue_4) (Collision|SphereTraceForObjects (+ (* (Math|Vector|GetForwardVector _returnvalue_3) -1e+02) _returnvalue) (+ _returnvalue (* (Math|Vector|GetForwardVector _returnvalue_3) 1e+02)) 24.0 (Utilities|Array|MakeArray "ObjectTypeQuery2" "ObjectTypeQuery3" "ObjectTypeQuery4" "ObjectTypeQuery6" "ObjectTypeQuery1") false (Utilities|Array|MakeArray _returnvalue_2) "None"))
  (if _returnvalue_4
    (Game|Damage|ApplyDamage (.HitActor (Collision|BreakHitResult _outhit)) 1e+02 0 _returnvalue_2)
    (return true)
    (else
      (return false))))