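; BP_LPAMG_Skin is a skin Blueprint, apparently for the LPAMG, that re-materials a referenced component according to its component type.
; ApplyTo looks up the given type in the Entries map by finding its index in the keys and reading the matching value.
; It then loops over that entry's ComponentData, setting each material on the reference by slot name, with no guard for a missing type.
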(fn Applyto
  (params (Reference :type Primitive%20Component%20Object%20Reference%20%28by%20ref%29) (Component%20Type :type Name))
  (Utilities|FlowControl|Sequence
    (:then_0
      (bind _keys (Utilities|Map|Keys (Variables|InfimaGames|Skin|GetEntries)))
      (bind _values (Utilities|Map|Values (Variables|InfimaGames|Skin|GetEntries)))
      (for _array_element (Utilities|Struct|BreakSkinComponent (Utilities|Array|Get(acopy) _values (Utilities|Array|FindItem _keys Component%20Type)))
        (Rendering|Material|SetMaterialbyName Reference (.MaterialSlotName (Utilities|Struct|BreakSkinComponentData _array_element)) (.Material (Utilities|Struct|BreakSkinComponentData _array_element))) ; This sets the material to the correct\nthing based on our map of entries.
      ))
    (:then_1
      (return))))