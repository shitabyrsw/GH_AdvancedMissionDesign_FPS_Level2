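; BP_Shield is a damageable shield actor that cycles off and on, and is destroyed when its health runs out.
; Tick drives the cycle through chained Delays, toggling AbsorbArea collision between query-only and none.
; One timeline shrinks the shield mesh on deactivation and plays in reverse to expand it.
; The AbsorbArea overlap event is empty, and the damage-volume cast, destroy and sound logic is disconnected.
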(event OnComponentBeginOverlap(AbsorbArea)
  (params (OverlappedComponent :type Primitive%20Component%20Object%20Reference) (OtherActor :type Actor%20Object%20Reference) (OtherComp :type Primitive%20Component%20Object%20Reference) (OtherBodyIndex :type Integer) (bFromSweep :type Boolean) (SweepResult :type Hit%20Result%20Structure%20%28by%20ref%29)))

(event Custom|ExpandShield
  (bind _scale (Timeline|ShrinkTimeline ReverseFromEnd)
    (:Update
      (Transformation|SetRelativeScale3D (Variables|Default|GetShieldMesh) (Math|Conversions|ToVector(Float) _scale)))))

(event Custom|Activare
  (Collision|SetCollisionEnabled (Variables|Default|GetAbsorbArea) "QueryOnly")
  (CallFunction|ExpandShield))

(event Custom|Deactivate
  (Collision|SetCollisionEnabled (Variables|Default|GetAbsorbArea) "NoCollision")
  (CallFunction|ShrinkShield))

(event Custom|ShrinkShield
  (bind _scale (Timeline|ShrinkTimeline PlayFromStart)
    (:Update
      (Transformation|SetRelativeScale3D (Variables|Default|GetShieldMesh) (Math|Conversions|ToVector(Float) _scale)))))

(event EventBeginPlay)

(event Collision|EventActorBeginOverlap
  (params (OtherActor :type Actor%20Object%20Reference)))

(event EventTick
  (params (DeltaSeconds :type Float%20%28single-precision%29))
  (Utilities|FlowControl|Delay 5.0)
  (CallFunction|Deactivate)
  (Utilities|FlowControl|Delay 3.0)
  (CallFunction|Activare))

(event Game|Damage|EventAnyDamage
  (params (Damage :type Float%20%28single-precision%29) (DamageType :type Damage%20Type%20Object%20Reference) (InstigatedBy :type Controller%20Object%20Reference) (DamageCauser :type Actor%20Object%20Reference))
  (bind _output_get (Variables|Default|Sethealth (- (Variables|Default|Gethealth) Damage)))
  (if (<= _output_get 0.0)
    (CallFunction|Deactivate)
    (Actor|DestroyActor)))

(fn ConstructionScript)