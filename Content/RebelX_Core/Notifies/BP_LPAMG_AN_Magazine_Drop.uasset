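; Anim notify, shown as "Drop Magazine", that drops a magazine from the weapon owning the animated mesh.
; It gets the weapon's magazine mesh component through an LPAMG message call and, if valid, spawns a BP_LPAMG_Magazine actor at that component's world transform.
; The spawned actor copies the component's static mesh and materials so it matches the visible magazine.
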(fn GetNotifyName
  (return "Drop Magazine"))

(fn ReceivedNotify
  (params (MeshComp :type Skeletal%20Mesh%20Component%20Object%20Reference) (Animation :type Anim%20Sequence%20Base%20Object%20Reference) (EventReference :type Anim%20Notify%20Event%20Reference%20Structure%20%28by%20ref%29))
  (Utilities|FlowControl|Sequence
    (:then_0
      (LocalVariables|SetActor%20Weapon (Components|GetOwner MeshComp) :!pinned true) ; Cache Weapon.
      (bind _returnvalue (Class|BPILPAMGWEP|LPAMG-GetMeshComponentMagazine(Message) (LocalVariables|GetActor%20Weapon)))
      (bind _output_get (LocalVariables|SetMesh%20Component%20Magazine _returnvalue))
      (Utilities|IsValid _output_get
        (:Is%20Valid
          (bind _returnvalue_2 (Game|SpawnActorfromClass "/Game/RebelX_Core/Blueprints/Weapons/BP_LPAMG_Magazine.BP_LPAMG_Magazine_C" (Transformation|GetWorldTransform (LocalVariables|GetMesh%20Component%20Magazine)) "Undefined" "OverrideRootScale" 0 0 :!pinned true)) ; Spawn New Magazine. This drops the magazine, basically.
          (LocalVariables|SetMesh%20Magazine _returnvalue_2)
          (Components|StaticMesh|SetStaticMesh (Variables|/Game/RebelX_Core/Blueprints/Weapons/BP_LPAMG_Magazine.BP_LPAMG_Magazine_C|GetMesh%20Magazine (LocalVariables|GetMesh%20Magazine)) (Variables|/Script/Engine.StaticMeshComponent|GetStaticMesh (LocalVariables|GetMesh%20Component%20Magazine)) :!pinned true) ; Copy Static Mesh. Matches the visual magazine.
          (Utilities|FlowControl|Sequence
            (:then_0
              (for _index (range 0 (Rendering|Material|GetNumMaterials (Variables|/Game/RebelX_Core/Blueprints/Weapons/BP_LPAMG_Magazine.BP_LPAMG_Magazine_C|GetMesh%20Magazine (LocalVariables|GetMesh%20Magazine))))
                (Rendering|Material|SetMaterial (Variables|/Game/RebelX_Core/Blueprints/Weapons/BP_LPAMG_Magazine.BP_LPAMG_Magazine_C|GetMesh%20Magazine (LocalVariables|GetMesh%20Magazine)) _index (Rendering|Material|GetMaterial (LocalVariables|GetMesh%20Component%20Magazine) _index))))))))
    (:then_1
      (return true))))