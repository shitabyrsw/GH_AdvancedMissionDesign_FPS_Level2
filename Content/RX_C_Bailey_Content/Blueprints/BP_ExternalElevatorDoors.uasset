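; External elevator doors for one floor, with a child-actor call button that summons the linked elevator.
; On BeginPlay it binds to the button's press event, which calls the elevator to this door's floor number.
; Events open and close both doors with a timeline that lerps their relative scale rather than moving them, reversing to close.
; A separate event returns the button to its inactive state.
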(event Custom|DoorsOpen
  (bind _lerpalpha (Timeline|Door%20Movement Play)
    (:Update
      (Transformation|SetRelativeScale3D (Variables|Default|GetDoorRight) (Math|Vector|Lerp(Vector) (Variables|Default|GetClosedScale) (Variables|Default|GetOpenScale) _lerpalpha)))))

(event Custom|DoorsClose
  (bind _lerpalpha (Timeline|Door%20Movement Reverse)
    (:Update
      (Transformation|SetRelativeScale3D (Variables|Default|GetDoorRight) (Math|Vector|Lerp(Vector) (Variables|Default|GetClosedScale) (Variables|Default|GetOpenScale) _lerpalpha)))))

(event Custom|ResetButton
  (bind _asbp_elevator_button (Utilities|Casting|CastToBP_ElevatorButton (Variables|/Script/Engine.ChildActorComponent|GetChildActor (Variables|Default|GetCallButton))))
  (Default|Inactive _asbp_elevator_button))

(event Custom|CallButtonPressed
  (Default|CallElevatortoFloor (Variables|Default|GetElevator) (Variables|Default|GetFloor%20Number)))

(event EventBeginPlay
  (bind _asbp_elevator_button (Utilities|Casting|CastToBP_ElevatorButton (Variables|/Script/Engine.ChildActorComponent|GetChildActor (Variables|Default|GetCallButton))))
  (EventDispatchers|BindEventtoButtonPressed _asbp_elevator_button (delegate Custom|CallButtonPressed)))

(event Collision|EventActorBeginOverlap
  (params (OtherActor :type Actor%20Object%20Reference)))

(event EventTick
  (params (DeltaSeconds :type Float%20%28single-precision%29)))

(fn ConstructionScript)