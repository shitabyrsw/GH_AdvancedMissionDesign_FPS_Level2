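; Inventory component that tracks ammo by type, a grenade count and a capped list of carried weapons with an equipped index.
; ResetAmmo applies multipliers to max and starting ammo through AddAmmo, which clamps totals and registers new types.
; Ammo changes write struct copies back to the map and dispatch full or depleted events, while UnlimitedAmmo bypasses consumption.
; Weapon cycling wraps around, and adding at capacity replaces the equipped weapon.
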(event Custom|ResetAmmo
  ;[1 1 1] Reset Ammo
  (bind _keys (Utilities|Map|Keys (Variables|RebelX|InventoryComponent|Ammo|GetAmmo)))
  (for _array_element _keys
    (Utilities|Map|Add (Variables|RebelX|InventoryComponent|Ammo|GetAmmo) _array_element (Utilities|Struct|MakeS_Inv_Ammo (.Avalible (RebelX|InventoryComponent|Ammo|GetAmmoOfType _array_element)) (* (.MaxAllowed (RebelX|InventoryComponent|Ammo|GetAmmoOfType _array_element)) (Variables|RebelX|InventoryComponent|Ammo|GetMaxAmmoMultiplier%20)))) ; Update max ammo from modifyer
    (RebelX|InventoryComponent|Ammo|AddAmmo _array_element (* (Variables|RebelX|InventoryComponent|Ammo|GetStartingAmmoMultiplier%20) (/ (.MaxAllowed (RebelX|InventoryComponent|Ammo|GetAmmoOfType _array_element)) 4)))))

(fn AddAmmo
  (params (Ammo%20Type :type E_WeaponAmmoTypes%20Enum :default "NewEnumerator0") (Quantity :type Integer))
  (bind _ammo (Variables|RebelX|InventoryComponent|Ammo|GetAmmo))
  (bind _ammo_2 (Variables|RebelX|InventoryComponent|Ammo|GetAmmo))
  (bind _value (Utilities|Map|Find _ammo Ammo%20Type))
  (bind (_value_2 _returnvalue) (Utilities|Map|Find _ammo_2 Ammo%20Type))
  (bind (_avalible _maxallowed) (Utilities|Struct|BreakS_Inv_Ammo _value_2))
  (bind (_avalible_2 _maxallowed_2) (Utilities|Struct|BreakS_Inv_Ammo _value))
  (bind _returnvalue_2 (== _avalible_2 _maxallowed_2))
  (Utilities|FlowControl|Sequence
    (:then_0
      ;[1 1 1] Log Desired
      (CallFunction|DebugLog (Utilities|String|Append "Adding " (Utilities|String|EnumtoString Ammo%20Type) " Ammo" "(" (Utilities|String|ToString(Integer) Quantity) ")") "NewEnumerator0" "None" false))
    (:then_1
      ;[1 1 1] Add ammo to map
      (if _returnvalue
        (LocalVariables|SetTemp_PreviousAvalible _avalible) ; For calculating total actually added
        (bind _structout (Utilities|Struct|SetmembersinS_Inv_Ammo _value_2 (Math|Integer|Clamp(Integer) (+ _avalible Quantity) 0 _maxallowed)))
        (Utilities|Map|Add (Variables|RebelX|InventoryComponent|Ammo|GetAmmo) Ammo%20Type _structout) ; Update Map with copy
        (else
          ;[1 1 1] Add new ammo type
          (CallFunction|DebugLog "Adding new ammo type" "NewEnumerator0" "None" false)
          (Utilities|Map|Add (Variables|RebelX|InventoryComponent|Ammo|GetAmmo) Ammo%20Type (Utilities|Struct|MakeS_Inv_Ammo Quantity 100)) ; Update Map with copy
        )))
    (:then_2
      ;[1 1 1] Log new total ammo
      (CallFunction|DebugLog (Utilities|String|Append "New " (Utilities|String|EnumtoString Ammo%20Type) " Ammo" "(" (Utilities|String|ToString(Integer) (.Avalible (Utilities|Struct|BreakS_Inv_Ammo (.Value (Utilities|Map|Find (Variables|RebelX|InventoryComponent|Ammo|GetAmmo) Ammo%20Type))))) ")") "NewEnumerator0" "None" false))
    (:then_3
      ;[1 1 1] Dispatch if full
      (if _returnvalue_2
        (Default|CallAmmoFull Ammo%20Type)))
    (:then_4
      ;[1 1 1] Output results
      (return _returnvalue_2 (- _avalible_2 (LocalVariables|GetTemp_PreviousAvalible))))))

(fn ConsumeAmmo
  (params (AmmoType :type E_WeaponAmmoTypes%20Enum :default "NewEnumerator0") (AmountToConsume :type Integer))
  (bind _ammo (Variables|RebelX|InventoryComponent|Ammo|GetAmmo))
  (bind _ammo_2 (Variables|RebelX|InventoryComponent|Ammo|GetAmmo))
  (bind _value (Utilities|Map|Find _ammo AmmoType))
  (bind _value_2 (Utilities|Map|Find _ammo_2 AmmoType))
  (bind _avalible (Utilities|Struct|BreakS_Inv_Ammo _value_2))
  (bind (_avalible_2 _maxallowed) (Utilities|Struct|BreakS_Inv_Ammo _value))
  (bind _returnvalue (- _avalible AmountToConsume))
  (if (Variables|RebelX|InventoryComponent|Ammo|GetUnlimitedAmmo)
    (return AmountToConsume false 0)
    (else
      (Utilities|FlowControl|Sequence
        (:then_0
          ;[1 1 1] Log Desired
          (CallFunction|DebugLog (Utilities|String|Append "Consuming " (Utilities|String|EnumtoString AmmoType) " Ammo" "(" (Utilities|String|ToString(Integer) AmountToConsume) ")") "NewEnumerator0" "None" false))
        (:then_1
          ;[1 1 1] Check for missing ammo
          (if (< _returnvalue 0)
            (LocalVariables|SetTemp_TotalMissing (Math|Integer|Absolute(Integer) _returnvalue))))
        (:then_2
          ;[1 1 1] Consume Ammo
          (bind _structout (Utilities|Struct|SetmembersinS_Inv_Ammo (.Value (Utilities|Map|Find (Variables|RebelX|InventoryComponent|Ammo|GetAmmo) AmmoType)) (Math|Integer|Clamp(Integer) (- _avalible_2 AmountToConsume) 0 _maxallowed)))
          (Utilities|Map|Add (Variables|RebelX|InventoryComponent|Ammo|GetAmmo) AmmoType _structout) ; Update map with copy
        )
        (:then_3
          ;[1 1 1] Log resluts
          (CallFunction|DebugLog (Utilities|String|Append "Comsumed  " (Utilities|String|EnumtoString AmmoType) " Ammo" "(" (Utilities|String|ToString(Integer) (- AmountToConsume (LocalVariables|GetTemp_TotalMissing))) ")") "NewEnumerator0" "None" false))
        (:then_4
          ;[1 1 1] Dispatch if depleted
          (if (== (.Avalible (Utilities|Struct|BreakS_Inv_Ammo (.Value (Utilities|Map|Find (Variables|RebelX|InventoryComponent|Ammo|GetAmmo) AmmoType)))) 0)
            (Default|CallAmmoDepleted AmmoType)))
        (:then_5
          ;[1 1 1] Output Results
          (return (- AmountToConsume (LocalVariables|GetTemp_TotalMissing)) (> (LocalVariables|GetTemp_TotalMissing) 0) (LocalVariables|GetTemp_TotalMissing)))))))

(fn GetAmmoOfType
  (params (AmmoType :type E_WeaponAmmoTypes%20Enum :default "NewEnumerator0"))
  (bind _ammo (Variables|RebelX|InventoryComponent|Ammo|GetAmmo))
  (bind (_value _returnvalue) (Utilities|Map|Find _ammo AmmoType))
  (return (.avalible _value) (.maxallowed _value) _returnvalue))

(fn AddThrowable
  (params (Count :type Integer))
  (Variables|RebelX|InventoryComponent|Throwable|SetGrenades (+ Count (Variables|RebelX|InventoryComponent|Throwable|GetGrenades))))

(fn ConsumeThrowable
  (if (not (< (- (Variables|RebelX|InventoryComponent|Throwable|GetGrenades) 1) 0))
    (Math|Integer|DecrementInt (Variables|RebelX|InventoryComponent|Throwable|GetGrenades)
      (:%20%20
        (return true)))
    (else
      (return false))))

(fn CycleWeapon
  ;[1 1 1] Has weapon
  (if (Utilities|Array|IsValidIndex (Variables|RebelX|InventoryComponent|Weapon|GetWeapons) (Variables|RebelX|InventoryComponent|Weapon|GetEquiped%20Weapon))
    (if (Utilities|Array|IsValidIndex (Variables|RebelX|InventoryComponent|Weapon|GetWeapons) (+ (Variables|RebelX|InventoryComponent|Weapon|GetEquiped%20Weapon) 1))
      ;[1 1 1] Increment Index
      (Math|Integer|IncrementInt (Variables|RebelX|InventoryComponent|Weapon|GetEquiped%20Weapon)
        (:%20%20
          (return (Utilities|Array|Get(acopy) (Variables|RebelX|InventoryComponent|Weapon|GetWeapons) (Variables|RebelX|InventoryComponent|Weapon|GetEquiped%20Weapon)) false)))
      (else
        ;[1 1 1] Reset Index
        (Variables|RebelX|InventoryComponent|Weapon|SetEquiped%20Weapon 0)
        (return (Utilities|Array|Get(acopy) (Variables|RebelX|InventoryComponent|Weapon|GetWeapons) (Variables|RebelX|InventoryComponent|Weapon|GetEquiped%20Weapon)) false)))
    (else
      ;[1 1 1] Unarmed
      (return 0 true))))

(fn AddWeapon
  (params (Weapon :type BP%20LPAMG%20WEP%20Object%20Reference%20%28by%20ref%29))
  (bind _weapons (Variables|RebelX|InventoryComponent|Weapon|GetWeapons))
  (if (== (Utilities|Array|LastIndex _weapons) (- (Variables|RebelX|InventoryComponent|Weapon|GetMax%20Carried%20Weapons) 1))
    (Utilities|Array|SetArrayElem (Variables|RebelX|InventoryComponent|Weapon|GetWeapons) (Variables|RebelX|InventoryComponent|Weapon|GetEquiped%20Weapon) Weapon)
    (return true)
    (else
      (bind _returnvalue (Utilities|Array|Add _weapons Weapon))
      (Variables|RebelX|InventoryComponent|Weapon|SetEquiped%20Weapon _returnvalue)
      (return false))))

(fn GetWeapon
  (bind _weapons (Variables|RebelX|InventoryComponent|Weapon|GetWeapons))
  (bind _equiped_weapon (Variables|RebelX|InventoryComponent|Weapon|GetEquiped%20Weapon))
  (return (not (Utilities|Array|IsValidIndex _weapons _equiped_weapon)) (Utilities|Array|Get(acopy) _weapons _equiped_weapon) (Variables|RebelX|InventoryComponent|Weapon|GetEquiped%20Weapon)))