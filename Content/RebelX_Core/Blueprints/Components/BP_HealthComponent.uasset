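; Actor component that gives its owner health and a recharging shield.
; Damage drains the shield first, without overflow into health, pauses recharge and restarts it after a delay via timers.
; A looping timer refills the shield until full, then pauses itself.
; Dispatchers announce damage, healing, shield states and health depletion, while the low, half and full health calls are never reached.
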(event Custom|Event%20Take%20Damage
  (params (Damage :type Float%20%28double-precision%29) (Damage%20Type :type Damage%20Type%20Object%20Reference))
  ;[1 1 1] Take Damage
  (Utilities|FlowControl|Sequence
    (:then_0
      (Utilities|Time|PauseTimerbyHandle (Variables|RebelX|HealthComponent|Shield|GetShield%20Recharge%20Tick))
      (Utilities|Time|SetTimerbyEvent (delegate Custom|Event%20Start%20Recharge) (Variables|RebelX|HealthComponent|Shield|GetSheild%20Recharge%20Delay)))
    (:then_1
      (if (<= (Variables|RebelX|HealthComponent|Shield|GetShield%20Current) 0.0)
        (RebelX|HealthComponent|Health|ConsumeHealth Damage)
        (else
          (bind _new_shield (RebelX|HealthComponent|Shield|ConsumeShield Damage))
          (if (<= _new_shield 0.0)
            (Default|CallShieldBroken)))))
    (:then_2
      (Default|CallDamageTaken (Variables|RebelX|HealthComponent|Health|GetHealth))
      (Utilities|CheckHealth))))

(event Custom|Event%20Shield%20Recharge
  ;[1 1 1] Begin Play
  ;;[1 1 1] Shield Recharge Timer
  (Variables|RebelX|HealthComponent|Shield|SetShield%20Current (Math|Float|Clamp(Float) (+ (Variables|RebelX|HealthComponent|Shield|GetShield%20Current) (Variables|RebelX|HealthComponent|Shield|GetShield%20Recharge%20Rate)) 0.0 (Variables|RebelX|HealthComponent|Shield|GetMax%20Shield)))
  (Default|CallShieldRecharging)
  (if (>= (Variables|RebelX|HealthComponent|Shield|GetShield%20Current) (Variables|RebelX|HealthComponent|Shield|GetMax%20Shield))
    (Utilities|Time|PauseTimerbyHandle (Variables|RebelX|HealthComponent|Shield|GetShield%20Recharge%20Tick))
    (Default|CallShieldRecharched)))

(event Custom|Event%20Start%20Recharge
  ;[1 1 1] Take Damage
  (Utilities|Time|UnpauseTimerbyHandle (Variables|RebelX|HealthComponent|Shield|GetShield%20Recharge%20Tick))
  (Default|CallShieldRechargeStarted))

(event EventBeginPlay
  ;[1 1 1] Begin Play
  (Utilities|FlowControl|Sequence
    (:then_0
      ;;[1 1 1] Setup Varaibles
      (Variables|RebelX|HealthComponent|Health|SetHealth (Variables|RebelX|HealthComponent|Health|GetMax%20Health))
      (Variables|RebelX|HealthComponent|Shield|SetShield%20Current (Variables|RebelX|HealthComponent|Shield|GetMax%20Shield)))
    (:then_1
      ;;[1 1 1] Shield Recharge Timer
      (bind _returnvalue (Utilities|Time|SetTimerbyEvent (delegate Custom|Event%20Shield%20Recharge) 0.1 true))
      (Variables|RebelX|HealthComponent|Shield|SetShield%20Recharge%20Tick _returnvalue))))

(fn AddHealth
  (params (Health%20To%20Add :type Float%20%28double-precision%29))
  (bind _output_get (Variables|RebelX|HealthComponent|Health|SetHealth (Math|Float|Clamp(Float) (+ (Variables|RebelX|HealthComponent|Health|GetHealth) Health%20To%20Add) 0.0 (Variables|RebelX|HealthComponent|Health|GetMax%20Health))))
  (Utilities|CheckHealth)
  (Default|CallHealed)
  (return _output_get))

(fn ConsumeHealth
  (params (Health%20To%20Consume :type Float%20%28double-precision%29))
  (bind _output_get (Variables|RebelX|HealthComponent|Health|SetHealth (Math|Float|Clamp(Float) (- (Variables|RebelX|HealthComponent|Health|GetHealth) Health%20To%20Consume) 0.0 (Variables|RebelX|HealthComponent|Health|GetMax%20Health))))
  (Utilities|CheckHealth)
  (return _output_get))

(fn AddShield
  (params (Shield :type Float%20%28double-precision%29))
  (Variables|RebelX|HealthComponent|Shield|SetShield%20Current (Math|Float|Clamp(Float) (+ Shield (Variables|RebelX|HealthComponent|Shield|GetShield%20Current)) 0.0 (Variables|RebelX|HealthComponent|Shield|GetMax%20Shield))))

(fn ConsumeShield
  (params (Shield%20To%20Consume :type Float%20%28double-precision%29))
  (bind _output_get (Variables|RebelX|HealthComponent|Shield|SetShield%20Current (Math|Float|Clamp(Float) (- (Variables|RebelX|HealthComponent|Shield|GetShield%20Current) Shield%20To%20Consume) 0.0 (Variables|RebelX|HealthComponent|Shield|GetMax%20Shield))))
  (return _output_get))