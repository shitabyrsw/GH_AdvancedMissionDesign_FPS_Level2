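; Blueprint function library of LPAMG math helpers for rotators, transforms and random ranges.
; Rotators add, subtract, negate and convert to and from vectors component-wise, with X as roll, Y pitch and Z yaw.
; Transform helpers reuse these rotator functions; adding resets scale to one, while negating can optionally preserve scale.
; Random float and integer helpers read a vector's X and Y as minimum and maximum, truncating for integers.
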(fn LPAMG-AddRotators
  (params (A :type Rotator) (B :type Rotator))
  (bind (_roll _pitch _yaw) (Math|Rotator|BreakRotator A))
  (bind (_roll_2 _pitch_2 _yaw_2) (Math|Rotator|BreakRotator B))
  (return (Math|Rotator|MakeRotator (+ _roll _roll_2) (+ _pitch _pitch_2) (+ _yaw _yaw_2))))

(fn LPAMG-NegateRotator
  (params (A :type Rotator))
  (return (* A -1.0)))

(fn LPAMG-AddTransforms
  (params (A :type Transform) (B :type Transform))
  (bind (_location _rotation) (Math|Transform|BreakTransform A))
  (bind (_location_2 _rotation_2) (Math|Transform|BreakTransform B))
  (return (Math|Transform|MakeTransform (+ _location _location_2) (InfimaGames|FunctionLibraries|Math|Pure|LPAMG-AddRotators _rotation _rotation_2 (LocalVariables|Get__WorldContext)))))

(fn LPAMG-VectortoRotator
  (params (In :type Vector))
  (bind (_x _y _z) (Math|Vector|BreakVector In))
  (return (Math|Rotator|MakeRotator _x _y _z)))

(fn LPAMG-RotatortoVector
  (params (Value :type Rotator))
  (bind (_roll _pitch _yaw) (Math|Rotator|BreakRotator Value))
  (return (Math|Vector|MakeVector _roll _pitch _yaw)))

(fn LPAMG-RandomFloatinVectorRange
  (params (Range :type Vector%202D%20Structure))
  (bind (_x _y) (Math|Vector2D|BreakVector2D Range))
  (return (Math|Random|RandomFloatinRange _x _y)))

(fn LPAMG-RandomIntegerinVectorRange
  (params (Range :type Vector%202D%20Structure))
  (bind (_x _y) (Math|Vector2D|BreakVector2D Range))
  (return (Math|Random|RandomIntegerinRange (Math|Float|Truncate _x) (Math|Float|Truncate _y))))

(fn LPAMG-NegateTransform
  (params (In :type Transform) (Ignore%20Scale :type Boolean))
  (bind (_location _rotation _scale) (Math|Transform|BreakTransform In))
  (return (Math|Transform|MakeTransform (Math|Vector|NegateVector _location) (InfimaGames|FunctionLibraries|Math|Pure|LPAMG-NegateRotator _rotation (LocalVariables|Get__WorldContext)) (select Ignore%20Scale _scale (Math|Vector|NegateVector _scale)))))

(fn LPAMG-SubtractRotators
  (params (A :type Rotator) (B :type Rotator))
  (bind (_roll _pitch _yaw) (Math|Rotator|BreakRotator A))
  (bind ___worldcontext (LocalVariables|Get__WorldContext))
  (bind _returnvalue (InfimaGames|FunctionLibraries|Math|Pure|LPAMG-NegateRotator B ___worldcontext))
  (bind (_roll_2 _pitch_2 _yaw_2) (Math|Rotator|BreakRotator _returnvalue))
  (return (Math|Rotator|MakeRotator (+ _roll _roll_2) (+ _pitch _pitch_2) (+ _yaw _yaw_2))))