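; Ammo pickup that supplies a set quantity of one ammo type through interaction getter functions.
; The construction script shows either a rescaled generic ammo box or a mesh matching the ammo type, depending on a toggle.
; The getters return a type-to-quantity map, an interaction type, a type-specific crosshair prompt with an [E] pickup tooltip, and mark the item as consumable.
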(fn ConstructionScript
  (bind _ammomesh (Variables|Default|GetAmmoMesh))
  (if (Variables|RebelX|Pickup|Ammo|GetUseAmmoBoxMesh)
    (Components|StaticMesh|SetStaticMesh _ammomesh "/Game/RebelX_Core/Props/Weapons/Ammo/SM_Weapons_Ammo_Box.SM_Weapons_Ammo_Box")
    (Transformation|SetWorldScale3D _ammomesh (Math|Vector|MakeVector 0.25 0.5 0.25))
    (else
      (Components|StaticMesh|SetStaticMesh (Variables|Default|GetAmmoMesh) (Utilities|Select :Index (Variables|RebelX|Pickup|Ammo|GetAmmoType) :NewEnumerator0 "/Game/RebelX_Core/Props/Weapons/Ammo/SM_Weapons_Ammo_Pistols.SM_Weapons_Ammo_Pistols" :NewEnumerator7 "/Game/RebelX_Core/Props/Weapons/Ammo/SM_Weapons_Ammo_Revolvers.SM_Weapons_Ammo_Revolvers" :NewEnumerator3 "/Game/RebelX_Core/Props/Weapons/Ammo/SM_Weapons_Ammo_Rifles.SM_Weapons_Ammo_Rifles" :NewEnumerator6 "/Game/RebelX_Core/Props/Weapons/Ammo/SM_Weapons_Ammo_LMGs.SM_Weapons_Ammo_LMGs" :NewEnumerator1 "/Game/RebelX_Core/Props/Weapons/Ammo/SM_Weapons_Ammo_SMGs.SM_Weapons_Ammo_SMGs" :NewEnumerator2 "/Game/RebelX_Core/Props/Weapons/Ammo/SM_Weapons_Ammo_Shotguns.SM_Weapons_Ammo_Shotguns" :NewEnumerator4 "/Game/RebelX_Core/Props/Weapons/Ammo/SM_Weapons_Ammo_Snipers.SM_Weapons_Ammo_Snipers" :NewEnumerator5 "/Game/RebelX_Core/Weapons/LRAF9/Meshes/SM_LPAMG_LRAF9_Rocket.SM_LPAMG_LRAF9_Rocket")))))

(fn GetAmmoInfo
  (return true (Utilities|Map|MakeMap (Variables|RebelX|Pickup|Ammo|GetAmmoType) (Variables|RebelX|Pickup|Ammo|GetAmmoQuantity))))

(fn GetInteractionType
  (return true "NewEnumerator1"))

(fn GetCrosshairPrompt
  (return (Utilities|Text|FormatText "{type} AMMO" (Utilities|Select :Index (Variables|RebelX|Pickup|Ammo|GetAmmoType) :NewEnumerator0 "PISTOL" :NewEnumerator7 "REVOLVER" :NewEnumerator3 "RIFLE" :NewEnumerator6 "LMG" :NewEnumerator1 "SMG" :NewEnumerator2 "SHOTGUN" :NewEnumerator4 "SNIPER" :NewEnumerator5 "LAUNCHER")) "[E] PICKUP"))

(fn GetIsConsumeable
  (return true))