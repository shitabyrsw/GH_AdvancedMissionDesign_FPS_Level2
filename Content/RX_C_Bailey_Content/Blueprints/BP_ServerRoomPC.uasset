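; Interactable server room PC that runs a timed upload objective, which stalls while enemies are inside its checker box.
; Activation creates a progress widget and starts looping timers that advance progress and poll for BP_Master_Enemy overlaps, pausing the upload during interruptions.
; Dispatchers announce start, halfway and completion.
; Timelines lerp the monitor material and rect light between red and green for uploading and completion, with audio cues.
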(event Custom|AddProgress
  ;[1 1 1] Increases Progress Bar
  (bind _output_get (Variables|Default|SetProgress (+ (Variables|Default|GetProgress) 1.0)))
  (if (>= _output_get 1e+02)
    (CallFunction|ProgressComplete)
    (elif (>= _output_get 5e+01)
      (Utilities|FlowControl|DoOnce false
        (:Completed
          (Default|CallServerDefHalfway))))))

(event Custom|Enemy%20Check
  (bind _wbl_progressbar (Variables|Default|GetWBL_ProgressBar))
  (bind _progress_timer (Variables|Default|GetProgress%20Timer))
  ;[1 1 1] Check for Enemies in area
  (if (> (Utilities|Array|Length (Collision|GetOverlappingActors (Variables|Default|GetEnemyChecker) "/Game/RebelX_Core/Blueprints/AI/BP_Master_Enemy.BP_Master_Enemy_C" :!class /Script/Engine.PrimitiveComponent)) 0)
    (Utilities|Time|PauseTimerbyHandle _progress_timer)
    (Variables|/Game/RX_C_Bailey_Content/Widgets/WBP_UploadProgress.WBP_UploadProgress_C|SetInterrupted _wbl_progressbar true)
    (else
      (Utilities|Time|UnpauseTimerbyHandle _progress_timer)
      (Variables|/Game/RX_C_Bailey_Content/Widgets/WBP_UploadProgress.WBP_UploadProgress_C|SetInterrupted _wbl_progressbar false))))

(event Custom|UpdateLightColor
  (bind _lightcolour (Variables|Default|GetLightColour))
  ;[1 1 1] Update Light Colour Event
  (Rendering|Material|SetVectorParameterValue (Variables|Default|GetLight%20Material) "SecondaryColor" _lightcolour :!class /Script/Engine.MaterialInstanceDynamic)
  (Rendering|Components|Light|SetLightColor (Variables|Default|GetRectLight) _lightcolour true))

(event Custom|Progress%20Complete
  ;[1 1 1] Complete Upload
  (Utilities|Time|ClearandInvalidateTimerbyHandle (Variables|Default|GetEnemy%20Checker%20Timer))
  (Utilities|Time|ClearandInvalidateTimerbyHandle (Variables|Default|GetProgress%20Timer))
  (Audio|Components|Audio|Stop (Variables|Default|GetUploading%20screen))
  (Audio|Components|Audio|Play (Variables|Default|GetScreenColour%20Change))
  (Default|CallProgressComplete)
  (Audio|Components|Audio|Play (Variables|Default|GetAudio) 0.0)
  (Utilities|FlowControl|Delay 4.0)
  (Widget|RemovefromParent (Variables|Default|GetWBL_ProgressBar)))

(event EventBeginPlay)

(event Collision|EventActorBeginOverlap
  (params (OtherActor :type Actor%20Object%20Reference)))

(event EventTick
  (params (DeltaSeconds :type Float%20%28single-precision%29)))

(event EventActivateSceneObject
  (Audio|Components|Audio|Play (Variables|Default|GetAudio1) 0.0)
  (Default|CallServerDefStarted)
  (Utilities|FlowControl|DoOnce false
    (:Completed
      (Utilities|FlowControl|Sequence
        (:then_0
          (Audio|Components|Audio|Play (Variables|Default|GetUploading%20screen)))
        (:then_1
          ;[1 1 1] Create Progress bar Widget
          (bind _returnvalue (UserInterface|CreateWidget "/Game/RX_C_Bailey_Content/Widgets/WBP_UploadProgress.WBP_UploadProgress_C" (Game|GetPlayerController 0) self))
          (bind _output_get (Variables|Default|SetWBL_ProgressBar _returnvalue))
          (UserInterface|Viewport|AddtoViewport _output_get 0))
        (:then_2
          (bind _returnvalue_2 (Utilities|Time|SetTimerbyEvent (delegate Custom|AddProgress) 0.5 true))
          (Variables|Default|SetProgress%20Timer _returnvalue_2)
          (bind _returnvalue_3 (Utilities|Time|SetTimerbyEvent (delegate Custom|Enemy%20Check) 0.5 true))
          (Variables|Default|SetEnemy%20Checker%20Timer _returnvalue_3))
        (:then_3
          (Variables|Default|SetInteraction%20Message "")
          (Variables|Default|SetCan%20Interact false))))))

(fn ConstructionScript
  (bind _enemychecker (Variables|Default|GetEnemyChecker))
  (|CallParentFunction)
  (bind _returnvalue (Rendering|Material|CreateDynamicMaterialInstance (Variables|Default|GetMonitor) 1 "/Game/RebelX_Core/Environment/Materials/MI_LightSurface.MI_LightSurface" "SecondaryColor" :!class /Script/Engine.PrimitiveComponent))
  (Variables|Default|SetLight%20Material _returnvalue)
  (Rendering|Material|SetVectorParameterValue (Variables|Default|GetLight%20Material) "SecondaryColor" (Variables|Default|GetLightColour) :!class /Script/Engine.MaterialInstanceDynamic)
  (Transformation|SetRelativeLocation _enemychecker (Variables|Default|GetLocationEnemyChecker) false false)
  (Components|Box|SetBoxExtent _enemychecker (Variables|Default|GetBox%20Extent%20EnemyChecker) true))

(fn GetInteractionType
  (return (Variables|Default|GetCan%20Interact) "NewEnumerator2"))

(fn GetCrosshairPrompt
  (return (Variables|Default|GetInteraction%20Message) "[E] Use"))