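; Anim notify that shows or hides the reserve magazine on an animated low-poly weapon during an animation.
; It asks the mesh component's owner for its weapon actor through an interface message, then passes its Visibility setting to that weapon via SetReserveMagazineVisibilityMessage.
; It displays as "Set Reserve Magazine Visibility (Art Pack)" in the animation editor.
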(fn ReceivedNotify
  (params (MeshComp :type Skeletal%20Mesh%20Component%20Object%20Reference) (Animation :type Anim%20Sequence%20Base%20Object%20Reference) (EventReference :type Anim%20Notify%20Event%20Reference%20Structure%20%28by%20ref%29))
  (Utilities|FlowControl|Sequence
    (:then_0
      (Utilities|IsValid MeshComp
        (:Is%20Valid
          (bind _returnvalue (Class|BPILPAMGPCH|LPAMG-GetActorAnimatedLowPolyWeapon(Message) (Components|GetOwner MeshComp)))
          (bind _output_get (LocalVariables|SetActor%20Weapon _returnvalue))
          (Utilities|IsValid _output_get
            (:Is%20Valid
              (Class|BPILPAMGMagazineReserverTarget|SetReserveMagazineVisibility(Message) (LocalVariables|GetActor%20Weapon) (Variables|Default|GetVisibility)))))))
    (:then_1
      (return true))))

(fn GetNotifyName
  (return "Set Reserve Magazine Visibility (Art Pack)"))