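; Damage volume actor that repeatedly damages any Characters standing inside its Box component.
; A Character beginning overlap starts a looping timer, if none is running, at the DamageTickDuration interval.
; Each tick applies DamagePerTick to every overlapping Character, with the volume as damage causer.
; When an overlap ends and no Characters remain, the timer is cleared and invalidated.
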(event OnComponentBeginOverlap(Box)
  (params (OverlappedComponent :type Primitive%20Component%20Object%20Reference) (OtherActor :type Actor%20Object%20Reference) (OtherComp :type Primitive%20Component%20Object%20Reference) (OtherBodyIndex :type Integer) (bFromSweep :type Boolean) (SweepResult :type Hit%20Result%20Structure%20%28by%20ref%29))
  ;[1 1 1] On overlap with charachter, start damage tick
  (if (not (Utilities|Time|IsValidTimerHandle (Variables|RebelX|DamageVolume|GetDamage%20Tick%20Timer)))
    (Utilities|Casting|CastToCharacter OtherActor)
    (bind _returnvalue (Utilities|Time|SetTimerbyEvent (delegate Custom|Event%20Damage%20Tick) (Variables|RebelX|DamageVolume|GetDamage%20Tick%20Duration) true))
    (Variables|RebelX|DamageVolume|SetDamage%20Tick%20Timer _returnvalue)))

(event OnComponentEndOverlap(Box)
  (params (OverlappedComponent :type Primitive%20Component%20Object%20Reference) (OtherActor :type Actor%20Object%20Reference) (OtherComp :type Primitive%20Component%20Object%20Reference) (OtherBodyIndex :type Integer))
  ;[1 1 1] Stop timer if no overlapps with charachter.
  (if (not (Utilities|Array|IsValidIndex (Collision|GetOverlappingActors "/Script/Engine.Character" :!class /Script/Engine.Actor)))
    (Utilities|Time|ClearandInvalidateTimerbyHandle (Variables|RebelX|DamageVolume|GetDamage%20Tick%20Timer))))

(event Custom|Event%20Damage%20Tick
  ;[1 1 1] Damge tick, applies damage to overlapped charachters.
  (for _array_element (Collision|GetOverlappingActors "/Script/Engine.Character" :!class /Script/Engine.Actor)
    (Game|Damage|ApplyDamage _array_element (Variables|RebelX|DamageVolume|GetDamage%20Per%20Tick) 0 self)))

(fn ConstructionScript)