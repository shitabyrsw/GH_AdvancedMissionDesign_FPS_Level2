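; AI enemy soldier character that fights with a child-actor weapon spawned from WeaponClass and reports its ammo type to the Blackboard.
; Fire and reload events drive the weapon component, playing montages supplied by the weapon, with shots randomized in a cone around control rotation.
; Alerting recolors its point light; death unpossesses it, ragdolls the mesh and destroys it after a delay.
; LPAMG animation interface getters mostly return fixed defaults.
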(event WeaponProjectileFired(BP_WeaponComponent_New)
  (bind _returnvalue (Class|BPILPAMGWEP|LPAMG-GetThirdPersonMontageCharacterFire(Message) (Variables|/Script/Engine.ChildActorComponent|GetChildActor (Variables|Default|GetChildActor))))
  (Animation|Montage|PlayMontage (Variables|Character|GetMesh) _returnvalue))

(event WeaponReloadStarted(BP_WeaponComponent_New)
  ;[1 1 1] Reload Animation
  (Default|ReloadEnd (Variables|Default|GetBP_WeaponComponent_New)))

(event Custom|OnAlert
  ;[1 1 1] On Alert
)

(event EventBeginPlay
  (bind _self self)
  (bind _returnvalue (AI|GetAIController _self))
  (bind _returnvalue_2 (AI|GetBlackboard _returnvalue))
  ;[1 1 1] Begin Play
  (Utilities|FlowControl|Sequence
    (:then_0
      ;;[1 1 1] Load Weapon Data
      (Utilities|FlowControl|DelayUntilNextTick)
      (bind _weapon_data (Class|BPILPAMGWEP|GetWeaponData(Message) (Variables|/Script/Engine.ChildActorComponent|GetChildActor (Variables|Default|GetChildActor))))
      (Default|InitWeaponComponent (Variables|Default|GetBP_WeaponComponent_New))
      (Utilities|IsValid _returnvalue_2
        (:Is%20Valid
          (AI|Components|Blackboard|SetValueasEnum _returnvalue_2 (Utilities|Name|MakeLiteralName "WeaponType") (Variables|/Game/RebelX_Core/Blueprints/Data/Weapons/BP_RebelX_Weapon_Data.BP_RebelX_Weapon_Data_C|GetAmmo%20Type _weapon_data)))))
    (:then_2)))

(event EventFireStop
  ;[1 1 1] Reload Animation
  (Default|TriggerReleased (Variables|Default|GetBP_WeaponComponent_New)))

(event EventEnemyHealthDepleted
  (bind _pointlight (Variables|Default|GetPointLight))
  ;[1 1 1] Health Depleated
  (|CallParentFunction)
  (Utilities|FlowControl|DoOnce false
    (:Completed
      (if (CallFunction|IsAIControllerValid)
        (Utilities|FlowControl|Sequence
          (:then_1
            (Pawn|UnPossess (AI|GetAIController self))
            (CallFunction|FireStop)
            (Audio|PlaySoundatLocation "/Game/RebelX_Core/Audio/Droid/SC_Droid_Death.SC_Droid_Death" (Transformation|GetActorLocation) "0, 0, 0" 1.0 1.0 0.0 0 0 0 0)
            (Utilities|IsValid _pointlight
              (:Is%20Valid
                (Components|DestroyComponent _pointlight))))
          (:then_2
            (Collision|SetCollisionProfileName (Variables|Character|GetMesh) "PhysicsActor" true :!class /Script/Engine.PrimitiveComponent)
            (Class|SkeletalMeshComponent|SetAllBodiesSimulatePhysics (Variables|Character|GetMesh) true)
            (Collision|SetCollisionResponsetoChannel (Variables|Character|GetMesh) "ECC_Pawn" "ECR_Ignore"))
          (:then_3
            (Utilities|FlowControl|Delay 3.0)
            (Actor|DestroyActor)))))))

(event EventFireStart
  ;[1 1 1] Reload Animation
  (Default|TriggerPressed (Variables|Default|GetBP_WeaponComponent_New)))

(event EventReload
  (Default|ReloadStart (Variables|Default|GetBP_WeaponComponent_New))
  (bind _returnvalue (Class|BPILPAMGWEP|LPAMG-GetThirdPersonMontageCharacterReload(Message) (Variables|/Script/Engine.ChildActorComponent|GetChildActor (Variables|Default|GetChildActor))))
  (Utilities|IsValid _returnvalue
    (:Is%20Valid
      (Animation|Montage|PlayMontage (Variables|Character|GetMesh) _returnvalue
        (:OnCompleted
          (Default|ReloadEnd (Variables|Default|GetBP_WeaponComponent_New)))))
    (:Is%20Not%20Valid
      (CallFunction|DebugLog "No reload montage found for phird person weapon animations" "NewEnumerator2" "None" false))))

(event EventCrouchStart
  (Character|Crouch))

(event EventCrouchEnd
  (Character|UnCrouch))

(event Game|Damage|EventAnyDamage
  (params (Damage :type Float%20%28single-precision%29) (DamageType :type Damage%20Type%20Object%20Reference) (InstigatedBy :type Controller%20Object%20Reference) (DamageCauser :type Actor%20Object%20Reference))
  (|CallParentFunction Damage DamageType InstigatedBy DamageCauser))

(event EventAlerted
  (bind _pointlight (Variables|Default|GetPointLight))
  (Utilities|IsValid _pointlight
    (:Is%20Valid
      (Rendering|Components|Light|SetLightColor _pointlight "(R=1.000000,G=0.250980,B=0.000000,A=1.000000)" true))))

(fn ConstructionScript
  (ChildActorComponent|SetChildActorClass (Variables|Default|GetChildActor) (Variables|Weapon|GetWeaponClass))
  (Default|InitWeaponComponent (Variables|Default|GetBP_WeaponComponent_New)))

(fn GetAIWeaponActor
  (return (Variables|/Script/Engine.ChildActorComponent|GetChildActor (Variables|Default|GetChildActor))))

(fn GetAIInventoryComponent
  (return (Variables|Default|GetBP_InventoryComponent)))

(fn GetAIWeaponComponent
  (return (Variables|Default|GetBP_WeaponComponent_New)))

(fn GetGrenadeCookDuration
  (return 0.0 0.0))

(fn GetHealthComponent
  (return 0))

(fn GetInteractActor
  (return 0))

(fn GetInventoryComponent
  (return (Variables|Default|GetBP_InventoryComponent)))

(fn GetProjectileFireLocation&Rotation
  (return (Transformation|GetWorldLocation (Variables|Default|GetChildActor)) (Math|Conversions|RotationFromXVector (Math|Random|RandomUnitVectorinConeinDegrees (Math|Vector|GetForwardVector (Pawn|GetControlRotation :!class /Script/Engine.Pawn)) 5.0))))

(fn GetWeaponComponent
  (return (Variables|Default|GetBP_WeaponComponent_New)))

(fn LPAMG-GetActorAnimatedLowPolyWeapon
  (return (Variables|/Script/Engine.ChildActorComponent|GetChildActor (Variables|Default|GetChildActor))))

(fn LPAMG-GetAnimationNameText
  (return ""))

(fn LPAMG-GetCameraComponent
  (return 0))

(fn LPAMG-GetInputValueLookHorizontal
  (return 0.0))

(fn LPAMG-GetInputValueLookVertical
  (return 0.0))

(fn LPAMG-GetInputValueMovementHorizontal
  (return 0.0))

(fn LPAMG-GetInputValueMovementVertical
  (return 0.0))

(fn LPAMG-GetOffsettingAmplitudeLocation
  (return 0.0))

(fn LPAMG-GetOffsettingAmplitudeRotation
  (return 0.0))

(fn LPAMG-GetTimeFiring
  (return 2.0))

(fn LPAMG-GetWeaponOffsetAimingLocation
  (return "0, 0, 0"))

(fn LPAMG-GetWeaponOffsetAimingRotation
  (return "0, 0, 0"))

(fn LPAMG-GetWeaponOffsetRunningLocation
  (return "0, 0, 0"))

(fn LPAMG-GetWeaponOffsetRunningRotation
  (return "0, 0, 0"))

(fn LPAMG-GetWeaponOffsetStandingLocation
  (return "0, 0, 0"))

(fn LPAMG-GetWeaponOffsetStandingRotation
  (return "0, 0, 0"))

(fn LPAMG-IsAiming
  (return false))

(fn LPAMG-IsCameraAnimated
  (return false))

(fn LPAMG-IsCrouching
  (return false))

(fn LPAMG-IsFirstPerson
  (return false))

(fn LPAMG-IsHolstered
  (return false))

(fn LPAMG-IsInspecting
  (return false))

(fn LPAMG-IsJumping
  (return false))

(fn LPAMG-IsLockedinFirstPerson
  (return false))

(fn LPAMG-IsLowered
  (return false))

(fn LPAMG-IsOffsettingLocation
  (return false))

(fn LPAMG-IsRunning
  (return false))

(fn LPAMG-IsTacticalSprinting
  (return false))

(fn LPAMG-IsUnarmed
  (return false))

(fn LPAMG-IsMoving
  (return false))