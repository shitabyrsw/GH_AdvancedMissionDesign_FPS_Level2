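; BP_CH_WeaponInspections records which weapon classes have been encountered, apparently as state for weapon inspections.
; It keeps a WeaponClassesEncountered collection with functions to query it, add a class only if absent, and clear it.
; The inspection behavior itself is not in this Blueprint, which only holds and manages that record.
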(fn HasEncounteredWeaponClass
  (params (Weapon%20Class :type BP%20LPAMG%20WEP%20Class%20Reference%20%28by%20ref%29))
  (return (Utilities|Array|ContainsItem (Variables|Default|GetWeapon%20Classes%20Encountered) Weapon%20Class)))

(fn AddEncounteredWeaponClass
  (params (Weapon%20Class :type BP%20LPAMG%20WEP%20Class%20Reference%20%28by%20ref%29))
  (bind _weapon_classes_encountered (Variables|Default|GetWeapon%20Classes%20Encountered))
  (if (Utilities|Array|ContainsItem _weapon_classes_encountered Weapon%20Class)
    _
    (else
      (Utilities|Array|Add _weapon_classes_encountered Weapon%20Class)))
  (return))

(fn ClearEncounteredWeapons
  (Utilities|Array|Clear (Variables|Default|GetWeapon%20Classes%20Encountered)))